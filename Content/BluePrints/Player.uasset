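; Player Blueprint that nudges itself in fixed world-space steps on W, A, S and D presses.
; Each key passes an offset to Move, which shifts the root component without sweep, increments TimesMoved and prints the count.
; BeginPlay separately runs an integer range check on Score and prints a green True or red False.
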(event EventBeginPlay
  (if (Math|Integer|InRange(Integer) (Variables|Default|GetScore) 5 10)
    (Development|PrintString "True" true true "(R=0.240057,G=1.000000,B=0.203346,A=1.000000)")
    (else
      (Development|PrintString "False" true true "(R=1.000000,G=0.000000,B=0.000000,A=1.000000)"))))

(event Input|KeyboardEvents|W
  (params (Key :type Key%20Structure :default "None"))
  (:Pressed
    (CallFunction|Move "10.000000, 0, 0")))

(event Input|KeyboardEvents|S
  (params (Key :type Key%20Structure :default "None"))
  (:Pressed
    (CallFunction|Move "-10.000000, 0, 0")))

(event Input|KeyboardEvents|A
  (params (Key :type Key%20Structure :default "None"))
  (:Pressed
    (CallFunction|Move "0,-10.000000, 0")))

(event Input|KeyboardEvents|D
  (params (Key :type Key%20Structure :default "None"))
  (:Pressed
    (CallFunction|Move "0,10.000000, 0")))

(fn ConstructionScript)

(fn Move
  (params (DeltaLocation :type Vector))
  (Transformation|AddWorldOffset (Variables|Default|GetDefaultSceneRoot) DeltaLocation false false)
  (bind _output_get (Variables|Default|SetTimesMoved (+ (Variables|Default|GetTimesMoved) 1)))
  (Development|PrintString (Utilities|String|ToString(Integer) _output_get)))